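; BP_Checkpoint is a level-end trigger that declares victory and moves the player to the next level.
; When a locally controlled pawn overlaps it, it shows victory text through the BoxHUD widget, plays a victory sound and starts a short timer.
; The timer event hides the text and opens the level named in NextLevelName, or quits the game if that name is empty.
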(event `self.ReceiveBeginPlay`)

(event `self.ReceiveActorBeginOverlap`
  (params (OtherActor :type "Actor Object Reference"))
  (bind _aspawn (cast `Pawn` OtherActor))
  (bind _returnvalue (`Pawn.GetController` _aspawn))
  (if (`Controller.IsLocalPlayerController` _returnvalue)
    (bind _asplayer_controller (cast `PlayerController` _returnvalue))
    (bind _asbox_hud (cast `BoxHUD` (`PlayerController.GetHUD` _asplayer_controller)))
    (`BoxHUDWidget.ShowVictoryText` (`BoxHUD.GetHUDWidget` _asbox_hud))
    (`KismetSystemLibrary.K2_SetTimerDelegate` (delegate `TransitNextLevel`) 2.0)
    (`GameplayStatics.PlaySound2D` (`self.VictorySound`) 1.0 1.0 0.0 null null)))

(event `TransitNextLevel`
  (bind _nextlevelname (`self.NextLevelName`))
  (if (`KismetStringLibrary.IsEmpty` _nextlevelname)
    (`KismetSystemLibrary.QuitGame` null "Quit")
    (else
      (`BoxHUDWidget.HideVictoryText` (`BoxHUD.GetHUDWidget` (stale `self.ReceiveActorBeginOverlap` _asbox_hud)))
      (`GameplayStatics.OpenLevel` (`KismetStringLibrary.Conv_StringToName` _nextlevelname)))))

(fn `UserConstructionScript`)