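; BP_Teleport is a teleporter prop that moves an overlapping pawn to a linked TeleportDestination, slightly above its origin.
; It acts only for pawns with a local player controller, and only when the destination is valid.
; Before the move it turns off overlap events on the destination's collision capsule, preventing an immediate bounce back, and a timer re-enables them two seconds later.
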(event `self.ReceiveActorBeginOverlap`
  (params (OtherActor :type "Actor Object Reference"))
  (bind _teleportdestination (`self.TeleportDestination`))
  (bind _aspawn (cast `Pawn` OtherActor))
  (if (`Controller.IsLocalPlayerController` (`Pawn.GetController` _aspawn))
    (if (`KismetSystemLibrary.IsValid` _teleportdestination)
      (`self.EnableTelport` _teleportdestination false)
      (`KismetSystemLibrary.K2_SetTimerDelegate` (delegate `CustomEvent`) 2.0)
      (`self.K2_SetActorLocation` OtherActor (+ (`self.K2_GetActorLocation` _teleportdestination) (0.0 0.0 50.0)) false false))))

(event `CustomEvent`
  (`self.EnableTelport` (`self.TeleportDestination`) true))

(fn `EnableTelport`
  (params (IsEnabled :type Boolean))
  (set `PrimitiveComponent.bGenerateOverlapEvents` IsEnabled (`self.CollisionCapsule`)))

(fn `UserConstructionScript`)